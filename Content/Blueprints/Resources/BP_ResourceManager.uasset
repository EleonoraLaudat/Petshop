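; BP_ResourceManager is a map-wide manager for resource spawn points, with initial resource generation currently limited to debug output.
; On BeginPlay it gathers every BP_ResourceSpawnPoint in the level into AllSpawnPoints.
; It then picks a random entry from the AllowedResources of each unoccupied point and prints its enum name.
; No resource is spawned and no point is marked occupied.
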(event EventBeginPlay
  (CallFunction|FindSpawnPoints)
  (CallFunction|GenerateInitialResources))

(event Collision|EventActorBeginOverlap
  (params (OtherActor :type Actor%20Object%20Reference)))

(event EventTick
  (params (DeltaSeconds :type Float%20%28single-precision%29)))

(fn ConstructionScript)

(fn FindSpawnPoints
  ;[1 1 1] Find all resource spawn points for the entire map
  (Utilities|Array|Clear (Variables|Default|GetAllSpawnPoints))
  (bind _outactors (Actor|GetAllActorsOfClass "/Game/Blueprints/Resources/BP_ResourceSpawnPoint.BP_ResourceSpawnPoint_C"))
  (for _array_element _outactors
    (bind _asbp_resource_spawn_point (Utilities|Casting|CastToBP_ResourceSpawnPoint _array_element))
    (Utilities|Array|Add (Variables|Default|GetAllSpawnPoints) _asbp_resource_spawn_point)))

(fn GenerateInitialResources
  (for _array_element (Variables|Default|GetAllSpawnPoints)
    (if (not (Variables|/Game/Blueprints/Resources/BP_ResourceSpawnPoint.BP_ResourceSpawnPoint_C|GetbOccupied _array_element))
      (if (> (Utilities|Array|Length (Variables|/Game/Blueprints/Resources/BP_ResourceSpawnPoint.BP_ResourceSpawnPoint_C|GetAllowedResources _array_element)) 0)
        (bind _output_get (LocalVariables|SetNewLocalVar (Utilities|Array|Get(acopy) (Variables|/Game/Blueprints/Resources/BP_ResourceSpawnPoint.BP_ResourceSpawnPoint_C|GetAllowedResources _array_element) (Math|Random|RandomIntegerinRange 0 (- (Utilities|Array|Length (Variables|/Game/Blueprints/Resources/BP_ResourceSpawnPoint.BP_ResourceSpawnPoint_C|GetAllowedResources _array_element)) 1)))))
        (Development|PrintString (Utilities|String|EnumtoString _output_get))))))